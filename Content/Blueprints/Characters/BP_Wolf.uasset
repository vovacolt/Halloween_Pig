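; Wolf character Blueprint that adds movement footstep audio and an attack trigger.
; BeginPlay creates a persistent 2D steps sound, which plays on any W, A, S or D press and stops on any release of those keys.
; The Attack input calls a server-named attack event that briefly pulses an Attack flag.
; A timed W_Wolf widget display is present but unconnected.
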(event `CustomEvent`)

(event `self.ReceiveBeginPlay`
  (bind _returnvalue (`GameplayStatics.CreateSound2D` "/Game/steps.steps" 0.4 1.0 0.0 null false false))
  (set `self.Sound` _returnvalue))

(event `Key|W`
  (params (Key :type "Key Structure"))
  (bind _sound (`self.Sound`))
  (:`Pressed`
    (`AudioComponent.Play` _sound 0.0 :!label _label))
  (:`Released`
    (`AudioComponent.Stop` _sound :!label _label_2)))

(event `Key|S`
  (params (Key :type "Key Structure"))
  (:`Pressed`
    (goto _label))
  (:`Released`
    (goto _label_2)))

(event `Key|A`
  (params (Key :type "Key Structure"))
  (:`Pressed`
    (goto _label))
  (:`Released`
    (goto _label_2)))

(event `Key|D`
  (params (Key :type "Key Structure"))
  (:`Pressed`
    (goto _label))
  (:`Released`
    (goto _label_2)))

(event `InputAction|Attack`
  (params (Key :type "Key Structure"))
  (:`Pressed`
    (`self.Server_Attack`)))

(event `Server_Attack`
  (set `self.Attack` true)
  (`KismetSystemLibrary.Delay` 0.2)
  (set `self.Attack` false))

(event `Key|LeftMouseButton`
  (params (Key :type "Key Structure")))

(event `Key|RightMouseButton`
  (params (Key :type "Key Structure")))

(fn `UserConstructionScript`
  (`parent.UserConstructionScript`))