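; BP_Deer is a deer character Blueprint with movement footstep audio and an attack that knocks barrels away.
; W, A, S and D presses play a 2D step sound created at BeginPlay, and any release stops it.
; Left click calls server-named events that pulse an Attack flag and launch overlapping Barrels forward and upward with physics impulses.
; The local impulse event is empty, and a similar StaticMeshActor impulse chain is unconnected.
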(event `self.ReceiveBeginPlay`
  (bind _returnvalue (`GameplayStatics.CreateSound2D` "/Game/steps.steps" 0.4 1.0 0.0 null false false))
  (set `self.Sound` _returnvalue))

(event `Key|W`
  (params (Key :type "Key Structure"))
  (bind _sound (`self.Sound`))
  (:`Pressed`
    (`AudioComponent.Play` _sound 0.0 :!label _label))
  (:`Released`
    (`AudioComponent.Stop` _sound :!label _label_2)))

(event `Key|S`
  (params (Key :type "Key Structure"))
  (:`Pressed`
    (goto _label))
  (:`Released`
    (goto _label_2)))

(event `Key|A`
  (params (Key :type "Key Structure"))
  (:`Pressed`
    (goto _label))
  (:`Released`
    (goto _label_2)))

(event `Key|D`
  (params (Key :type "Key Structure"))
  (:`Pressed`
    (goto _label))
  (:`Released`
    (goto _label_2)))

(event `Server_Attack`
  (set `self.Attack` true)
  (`KismetSystemLibrary.Delay` 0.2)
  (set `self.Attack` false))

(event `Key|LeftMouseButton`
  (params (Key :type "Key Structure"))
  (:`Pressed`
    (`|ExecutionSequence`
      (:`then_0`
        (`self.Server_Attack`))
      (:`then_1`
        (`self.Impulus_Server`))
      (:`then_2`
        (`self.Impulus_Local`)))))

(event `Impulus_Server`
  (bind (_returnvalue_x _returnvalue_y) (`KismetMathLibrary.BreakVector` (`SceneComponent.GetForwardVector` (`self.CapsuleComponent`))))
  (for _array_element (`PrimitiveComponent.GetOverlappingActors` (`self.Box`) null)
    (bind _asbarrel (cast `/Game/Barrel` _array_element))
    (bind _staticmesh (`/Game/Barrel.StaticMesh` _asbarrel))
    (`PrimitiveComponent.SetSimulatePhysics` _staticmesh true)
    (`PrimitiveComponent.AddImpulse` _staticmesh (`KismetMathLibrary.MakeVector` (* 1000 _returnvalue_x) (* 1000 _returnvalue_y) 100.0) "None" true)))

(event `Impulus_Local`)

(fn `UserConstructionScript`
  (`parent.UserConstructionScript`))